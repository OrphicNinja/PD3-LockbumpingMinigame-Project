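; Mod Blueprint that eases the lockbumping minigame while the Rush speed buff is active.
; Each Tick scans HUD buff widgets for the speed buff, setting RushActive from its visibility and removing it when hidden.
; Tick also updates all lockbumping widgets, forcing one ring during Rush and otherwise applying difficulty-based ring values.
; BeginPlay creates a lockbumping widget, but updates find widgets by class rather than through that reference.
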(event `self.ReceiveBeginPlay`
  ;[0 0 0] Creates lockbumping minigame widget reference
  (bind _returnvalue (`|CreateWidget` "/Game/UI/Widgets/HUD/WBP_UI_Widget_MiniGame_LockBumping.WBP_UI_Widget_MiniGame_LockBumping_C"))
  (set `self.LockBumping_Widget` _returnvalue)
  ;[0 0 0] Gets local player controller
  (set `self.PlayerController` (`SBZPlayerLibrary.GetLocalPlayerController`)))

(event `self.ReceiveTick`
  (params (DeltaSeconds :type "Float (single-precision)"))
  (`parent.ReceiveTick` DeltaSeconds)
  (`self.SetRushMinigameEffect`)
  ;[0 0 0] Gets Rush widget -> If widget is active, set RushActive to true
  (bind _foundwidgets (`WidgetBlueprintLibrary.GetAllWidgetsOfClass` "/Game/UI/Widgets/HUD/Buff/WBP_UI_HUD_Buff.WBP_UI_HUD_Buff_C" false))
  (for _array_element _foundwidgets
    (if (== (`SBZCharacterEffectWidget.BuffDataAsset` _array_element) "/Game/DataAssets/UICharacterEffects/DA_CharEffect_PlayerBuffSpeed.DA_CharEffect_PlayerBuffSpeed")
      (if (`SBZUIStatics.IsWidgetActuallyVisible` _array_element)
        (set `self.RushActive` true)
        (else
          (`Widget.RemoveFromParent` _array_element)
          (set `self.RushActive` false))))))

(event `SetRushMinigameEffect`
  ;[0 0 0] Gets lockbumping widget -> If RushActive is true, sets the number of rings needed to lockpick to 1 -> If RushActive is false, sets rings needed to lockpick based on difficulty
  (bind _foundwidgets (`WidgetBlueprintLibrary.GetAllWidgetsOfClass` "/Game/UI/Widgets/HUD/WBP_UI_Widget_MiniGame_LockBumping.WBP_UI_Widget_MiniGame_LockBumping_C" false))
  (for _array_element _foundwidgets
    (if (`self.RushActive`)
      (set `/Game/UI/Widgets/HUD/WBP_UI_Widget_MiniGame_LockBumping.NumOfRings` 1 _array_element)
      (else
        (bind _outputpins (`PD3HeistGameState.DifficultyBranch`))
        (`/Game/UI/Widgets/HUD/WBP_UI_Widget_MiniGame_LockBumping.SetRingSize&Values` _array_element _outputpins)))))

(fn `UserConstructionScript`)